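; BP_DoorTrigger1 is a trigger box that activates linked doors when the third-person character enters it, once it has been armed.
; On BeginPlay it binds TriggerInterruptor through EventLauncher, and that event hides the box and sets IsActionnable.
; While armed, each character overlap sends ActivateMessage to every BPControlDoor entry implementing BPI_Trigger.
; It combines an event binding for arming with interface messages for door activation.
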(event `self.ReceiveBeginPlay`
  (add `/Game/BluePrint/Application_CommunicationBP/BP_TriggerBoxes.TriggerBoxes` (`self.Event Launcher`) (delegate `TriggerInterruptor`)))

(event `TriggerInterruptor`
  (`SceneComponent.SetVisibility` (`self.Box`) false false)
  (set `self.IsActionnable` true))

(event `self.Box.OnComponentBeginOverlap`
  (params (OverlappedComponent :type "PrimitiveComponent Object Reference") (OtherActor :type "Actor Object Reference") (OtherComp :type "PrimitiveComponent Object Reference") (OtherBodyIndex :type Integer) (bFromSweep :type Boolean) (SweepResult :type "HitResult Structure (by ref)"))
  (if (`self.IsActionnable`)
    (cast `/Game/ThirdPerson/Blueprints/BP_ThirdPersonCharacter` OtherActor)
    (for _array_element (`self.BP_ControlDoor`)
      (if (`KismetSystemLibrary.DoesImplementInterface` _array_element "/Game/BluePrint/BPI_Trigger.BPI_Trigger_C")
        (message `/Game/BluePrint/BPI_Trigger.Activate` _array_element)))))

(fn `UserConstructionScript`)