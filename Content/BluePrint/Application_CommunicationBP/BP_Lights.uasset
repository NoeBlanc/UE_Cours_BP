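; BP_Lights is a light actor that turns its point light on when its door count reaches exactly three.
; It hides the light on BeginPlay, then relies on NumberIncrease and NumberDecrease, with no caller in this Blueprint, to adjust NumberOfDoors.
; Increasing shows the light at three, decreasing hides it at any other count, and both print debug messages.
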(event `self.ReceiveBeginPlay`
  (`SceneComponent.SetVisibility` (`self.PointLight`) false false))

(fn `NumberDecrease`
  (set `self.NumberOfDoors` (- (`self.NumberOfDoors`) 1))
  (`KismetSystemLibrary.PrintString` "on soustrait")
  (if (!= (`self.NumberOfDoors`) 3)
    (`SceneComponent.SetVisibility` (`self.PointLight`) false false)))

(fn `NumberIncrease`
  (bind _output_get (set `self.NumberOfDoors` (+ (`self.NumberOfDoors`) 1)))
  (`KismetSystemLibrary.PrintString` (`KismetStringLibrary.Concat_StrStr` "total porte :" (`KismetStringLibrary.Conv_IntToString` _output_get)))
  (if (== (`self.NumberOfDoors`) 3)
    (`SceneComponent.SetVisibility` (`self.PointLight`) true false)))

(fn `UserConstructionScript`)