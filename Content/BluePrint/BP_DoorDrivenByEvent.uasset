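; Door actor that toggles open and closed when an external event fires.
; On BeginPlay it binds ActivateDoor to the ActivateControllables event dispatcher on its EventLauncher reference, so the door reacts without polling.
; Each activation calls ToggleOpenClose, which checks the Cube's relative Y and snaps it between the origin and a sideways offset, with no animation or sweep.
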(event `self.ReceiveBeginPlay`
  (add `/Game/BluePrint/BP_TriggerByEvent.ActivateControllables` (`self.EventLauncher`) (delegate `ActivateDoor`)))

(event `ActivateDoor`
  (`self.ToggleOpenClose`))

(fn `ToggleOpenClose`
  (bind (_relativelocation_x _relativelocation_y) (`KismetMathLibrary.BreakVector` (`SceneComponent.RelativeLocation` (`self.Cube`))))
  (if (> _relativelocation_y 0.0)
    (`SceneComponent.K2_SetRelativeLocation` (`self.Cube`) (0.0 0.0 0.0) false false)
    (else
      (`SceneComponent.K2_SetRelativeLocation` (`self.Cube`) (0.0 100.0 0.0) false false))))

(fn `UserConstructionScript`)