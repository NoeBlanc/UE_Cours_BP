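; BP_Door is a sliding door actor that opens and closes in response to Activate and Desactivate events.
; Both events call ToggleOpenClose, so each one flips the current state rather than forcing open or closed.
; The toggle reads the Cube component's relative Y and snaps it between the origin and a sideways offset, with no sweep or animation.
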(event `/Game/BluePrint/BPI_Trigger.Activate`
  (`self.ToggleOpenClose`))

(event `/Game/BluePrint/BPI_Trigger.Desactivate`
  (`self.ToggleOpenClose`))

(fn `ToggleOpenClose`
  (bind (_relativelocation_x _relativelocation_y) (`KismetMathLibrary.BreakVector` (`SceneComponent.RelativeLocation` (`self.Cube`))))
  (if (> _relativelocation_y 0.0)
    (`SceneComponent.K2_SetRelativeLocation` (`self.Cube`) (0.0 0.0 0.0) false false)
    (else
      (`SceneComponent.K2_SetRelativeLocation` (`self.Cube`) (0.0 100.0 0.0) false false))))

(fn `UserConstructionScript`)